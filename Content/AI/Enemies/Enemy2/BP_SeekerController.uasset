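; BP_SeekerController is the AI controller for Seeker enemies and runs the BT_SeekerEnemy behavior tree on BeginPlay.
; Its ReportSighting event shares a sighting with the other Seekers by copying this controller's LastKnownLocation blackboard value into theirs.
; It finds them with GetAllActorsOfClass on BP_SeekerEnemy, skips its own pawn and stops at the first one whose controller fails the cast.
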(event `ReportSighting`
  (bind _lastknownlocationkey (`self.LastKnownLocationKey`))
  (bind _outactors (`GameplayStatics.GetAllActorsOfClass` "/Game/AI/Enemies/Enemy2/BP_SeekerEnemy.BP_SeekerEnemy_C"))
  (for _array_element _outactors
    (if (!= _array_element (`self.K2_GetPawn`))
      (bind _asbp_seeker_controller (cast `/Game/AI/Enemies/Enemy2/BP_SeekerController` (`AIBlueprintHelperLibrary.GetAIController` _array_element)))
      (`BlackboardComponent.SetValueAsVector` (`AIBlueprintHelperLibrary.GetBlackboard` _asbp_seeker_controller) _lastknownlocationkey (`BlackboardComponent.GetValueAsVector` (`AIBlueprintHelperLibrary.GetBlackboard` self) _lastknownlocationkey)))))

(event `self.ReceiveBeginPlay`
  (`self.RunBehaviorTree` "/Game/AI/Enemies/Enemy2/BT_SeekerEnemy.BT_SeekerEnemy"))

(fn `UserConstructionScript`)