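; Seeker enemy actor that detects the player through AI perception and is destroyed when it hits an AI_bot_Cat_1.
; On sensing the player, it spawns an influence marker at the stimulus location, writes target and last known location to the Blackboard, then reports the sighting to its BP_SeekerController.
; Losing the player clears only the target, leaving the last known location in place.
; Debug prints trace perception changes, and a disconnected location-update loop never runs.
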(event `self.ReceiveBeginPlay`)

(event `self.ReceiveHit`
  (params (MyComp :type "PrimitiveComponent Object Reference") (Other :type "Actor Object Reference") (OtherComp :type "PrimitiveComponent Object Reference") (bSelfMoved :type Boolean) (HitLocation :type "Vector Structure") (HitNormal :type "Vector Structure") (NormalImpulse :type "Vector Structure") (Hit :type "HitResult Structure (by ref)"))
  (cast `/Game/AI/Assistant/AI_bot_Cat_1` Other)
  (`self.K2_DestroyActor`))

(event `self.AIPerception.OnTargetPerceptionUpdated`
  (params (Actor :type "Actor Object Reference") (Stimulus :type "AIStimulus Structure"))
  (bind (_age _expirationage _strength _stimuluslocation _receiverlocation _tag _bsuccessfullysensed) (break `AIStimulus` Stimulus))
  (bind _returnvalue (`KismetStringLibrary.Conv_StringToName` "TargetActor"))
  (bind _blackboard (`AIController.Blackboard` (`AIBlueprintHelperLibrary.GetAIController` self)))
  (if _bsuccessfullysensed
    (bind _asbp_td_player (cast `/Game/AI/BP_TD_Player` Actor))
    (`KismetSystemLibrary.PrintString` "вижу")
    (`|SpawnActorFromClass` "/Game/AI/Enemies/Enemy2/BP_InfluenceMarker.BP_InfluenceMarker_C" (`KismetMathLibrary.Conv_VectorToTransform` _stimuluslocation) "Undefined" "OverrideRootScale" null null)
    (`BlackboardComponent.SetValueAsObject` _blackboard _returnvalue _asbp_td_player)
    (`KismetSystemLibrary.PrintString` "actor")
    (`BlackboardComponent.SetValueAsVector` _blackboard (`self.LastKnownLocationKey`) (`self.K2_GetActorLocation` _asbp_td_player))
    (bind _asbp_seeker_controller (cast `/Game/AI/Enemies/Enemy2/BP_SeekerController` (`self.GetController`)))
    (`/Game/AI/Enemies/Enemy2/BP_SeekerController.ReportSighting` _asbp_seeker_controller)
    (else
      (cast `/Game/AI/BP_TD_Player` Actor)
      (`BlackboardComponent.ClearValue` _blackboard _returnvalue)
      (`KismetSystemLibrary.PrintString` "не вижу"))))

(fn `UserConstructionScript`)